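; Base 3D text input field that registers itself with PC_controller_base when its cube is clicked.
; Per-key functions pass a glyph actor class to KeyBase, which spawns it, attaches it at LayoutPoint and advances the cursor by its SpaceSpan.
; Near EndObject, input is blocked, the cursor hides and the end marker shows unavailable.
; Backspace destroys the last glyph and restores cursor and marker; space bar is empty.
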(event `self.ReceiveBeginPlay`
  (`self.init_function`)
  (switch `/Game/HUI/BP/common/component/input/base/input_event_layout_enum` (`self.input_event_layout_enum`)))

(event `self.onclick_cube.OnClicked`
  (params (TouchedComponent :type "PrimitiveComponent Object Reference") (ButtonPressed :type "Key Structure"))
  ;[1 1 1] ransition to PC_controller_base
  (bind _aspc_controller_base (cast `/Game/HUI/BP/common/controll_BP/PC_controller_base` (`GameplayStatics.GetPlayerController` 0)))
  (set `/Game/HUI/BP/common/controll_BP/PC_controller_base.input_event_base_BP_temp` self _aspc_controller_base))

(fn `char_base_logic`
  (params (char_base_BP :type "/Game/HUI/BP/common/char_BP/base/char_base_BP Class Reference"))
  (locals (space_span :type "Float (double-precision)" :default 0.0))
  (bind _curcor_transform_temp_location (`KismetMathLibrary.BreakTransform` (`self.curcor_transform_temp`)))
  (bind (_curcor_transform_temp_location_2 _curcor_transform_temp_rotation _curcor_transform_temp_scale) (`KismetMathLibrary.BreakTransform` (`self.curcor_transform_temp`)))
  (bind _curcor_transform_temp (`self.curcor_transform_temp`))
  (bind _cursor (`self.cursor`))
  (bind _returnvalue (`SceneComponent.GetRelativeTransform` _cursor))
  (bind _returnvalue_2 (`|SpawnActorFromClass` char_base_BP (`KismetMathLibrary.MakeTransform` (+ _curcor_transform_temp_location_2 100.0) _curcor_transform_temp_rotation _curcor_transform_temp_scale) "Undefined" "OverrideRootScale" null null))
  (`SceneComponent.K2_SetRelativeLocation` (`/Game/HUI/BP/common/char_BP/base/char_base_BP.DefaultSceneRoot` _returnvalue_2) _curcor_transform_temp_location false false)
  (set `local.space_span` (`/Game/HUI/BP/common/char_BP/base/char_base_BP.space_span` _returnvalue_2))
  (`self.K2_AttachToComponent` _returnvalue_2 (`self.layout_point`) "None" "KeepRelative" "KeepRelative" "KeepRelative" true)
  (`KismetArrayLibrary.Array_Add` (`self.char_list`) _returnvalue_2)
  (bind _char_static_mesh (`/Game/HUI/BP/common/char_BP/base/char_base_BP.get_char_static_mesh` _returnvalue_2))
  (`PrimitiveComponent.SetMaterial` _char_static_mesh 0 (`self.char_material`))
  (`MeshComponent.SetScalarParameterValueOnMaterials` _char_static_mesh (`self.emissive color densy name`) (`self.input_body emissive color densy  value`))
  (bind _relativescale3d_x (`KismetMathLibrary.BreakVector` (`SceneComponent.RelativeScale3D` (`Actor.RootComponent` _returnvalue_2))))
  (bind _output_get (set `self.curcor_transform_temp` (`KismetMathLibrary.MakeTransform` (`KismetMathLibrary.MakeVector` (+ (* _relativescale3d_x (`local.space_span`)) (.x (.location _curcor_transform_temp))) (.y (.location _curcor_transform_temp)) (.z (.location _curcor_transform_temp))) (.rotation _curcor_transform_temp) (.scale _curcor_transform_temp))))
  ;[1 1 1] cursor position logic
  (`SceneComponent.K2_SetRelativeTransform` _cursor (`KismetMathLibrary.MakeTransform` (`KismetMathLibrary.MakeVector` (.x (.location _output_get)) (.y (.location _returnvalue)) (.z (.location _returnvalue))) (.rotation _returnvalue) (.scale _returnvalue)) false false))

(fn `init_function`
  (bind (_returnvalue_location _returnvalue_rotation _returnvalue_scale) (`KismetMathLibrary.BreakTransform` (`SceneComponent.GetRelativeTransform` (`self.layout_point`))))
  (`|ExecutionSequence`
    (:`then_0`
      ;[1 1 1] set char transform temp
      (set `self.curcor_transform_temp` (`KismetMathLibrary.MakeTransform` (0.0 0.0 0.0) _returnvalue_rotation _returnvalue_scale)))
    (:`then_1`
      ;[1 1 1] material
      (`self.set_input_body_material` null (`self.input_body emissive color densy  value`))
      (`self.set_input_border_material` null (`self.input_border emissive color densy  value`)))))

(fn `input_to_end`
  (returns (is_end :type Boolean))
  (bind _char_list (`self.char_list`))
  (bind _relativelocation_x (`KismetMathLibrary.BreakVector` (`SceneComponent.RelativeLocation` (`self.end_object`))))
  (bind _output (`|GetArrayItem` _char_list (- (`KismetArrayLibrary.Array_Length` _char_list) 1)))
  (`/Engine/EditorBlueprintResources/StandardMacros.IsValid` _output
    (:`Is Valid`
      (if (<= (- _relativelocation_x (.x (.location (`SceneComponent.GetRelativeTransform` (`/Game/HUI/BP/common/char_BP/base/char_base_BP.DefaultSceneRoot` _output))))) 200.0)
        (return true)
        (else
          (return false))))))

(fn `Key Base`
  (params (char_base_BP :type "/Game/HUI/BP/common/char_BP/base/char_base_BP Class Reference"))
  (bind _is_end (`self.input_to_end`))
  (if _is_end
    (`|ExecutionSequence`
      (:`then_0`
        ;[1 1 1] not available for end_object
        (bind _asend_object (cast `/Game/HUI/BP/common/component/input/base/end_object` (`ChildActorComponent.ChildActor` (`self.end_object`))))
        (`/Game/HUI/BP/common/component/input/base/end_object.material_for_not_available` _asend_object))
      (:`then_1`
        ;[1 1 1] cursor visibility is false
        (`SceneComponent.SetVisibility` (`self.cursor`) false false)))
    (else
      (`self.char_base_logic` char_base_BP))))

(fn `key_char_lower_a`
  (`self.Key Base` "/Game/HUI/BP/common/char_BP/char/lower/char_lower_a_BP.char_lower_a_BP_C"))

(fn `key_char_lower_b`
  (`self.Key Base` "/Game/HUI/BP/common/char_BP/char/lower/char_lower_b_BP.char_lower_b_BP_C"))

(fn `key_char_lower_c`
  (`self.Key Base` "/Game/HUI/BP/common/char_BP/char/lower/char_lower_c_BP.char_lower_c_BP_C"))

(fn `key_char_lower_d`
  (`self.Key Base` "/Game/HUI/BP/common/char_BP/char/lower/char_lower_d_BP.char_lower_d_BP_C"))

(fn `key_char_lower_e`
  (`self.Key Base` "/Game/HUI/BP/common/char_BP/char/lower/char_lower_e_BP.char_lower_e_BP_C"))

(fn `key_char_lower_f`
  (`self.Key Base` "/Game/HUI/BP/common/char_BP/char/lower/char_lower_f_BP.char_lower_f_BP_C"))

(fn `key_char_lower_g`
  (`self.Key Base` "/Game/HUI/BP/common/char_BP/char/lower/char_lower_g_BP.char_lower_g_BP_C"))

(fn `key_char_lower_h`
  (`self.Key Base` "/Game/HUI/BP/common/char_BP/char/lower/char_lower_h_BP.char_lower_h_BP_C"))

(fn `key_char_lower_i`
  (`self.Key Base` "/Game/HUI/BP/common/char_BP/char/lower/char_lower_i_BP.char_lower_i_BP_C"))

(fn `key_char_lower_j`
  (`self.Key Base` "/Game/HUI/BP/common/char_BP/char/lower/char_lower_j_BP.char_lower_j_BP_C"))

(fn `key_char_lower_k`
  (`self.Key Base` "/Game/HUI/BP/common/char_BP/char/lower/char_lower_k_BP.char_lower_k_BP_C"))

(fn `key_char_lower_l`
  (`self.Key Base` "/Game/HUI/BP/common/char_BP/char/lower/char_lower_l_BP.char_lower_l_BP_C"))

(fn `key_char_lower_m`
  (`self.Key Base` "/Game/HUI/BP/common/char_BP/char/lower/char_lower_m_BP.char_lower_m_BP_C"))

(fn `key_char_lower_n`
  (`self.Key Base` "/Game/HUI/BP/common/char_BP/char/lower/char_lower_n_BP.char_lower_n_BP_C"))

(fn `key_char_lower_o`
  (`self.Key Base` "/Game/HUI/BP/common/char_BP/char/lower/char_lower_o_BP.char_lower_o_BP_C"))

(fn `key_char_lower_p`
  (`self.Key Base` "/Game/HUI/BP/common/char_BP/char/lower/char_lower_p_BP.char_lower_p_BP_C"))

(fn `key_char_lower_q`
  (`self.Key Base` "/Game/HUI/BP/common/char_BP/char/lower/char_lower_q_BP.char_lower_q_BP_C"))

(fn `key_char_lower_r`
  (`self.Key Base` "/Game/HUI/BP/common/char_BP/char/lower/char_lower_r_BP.char_lower_r_BP_C"))

(fn `key_char_lower_s`
  (`self.Key Base` "/Game/HUI/BP/common/char_BP/char/lower/char_lower_s_BP.char_lower_s_BP_C"))

(fn `key_char_lower_t`
  (`self.Key Base` "/Game/HUI/BP/common/char_BP/char/lower/char_lower_t_BP.char_lower_t_BP_C"))

(fn `key_char_lower_u`
  (`self.Key Base` "/Game/HUI/BP/common/char_BP/char/lower/char_lower_u_BP.char_lower_u_BP_C"))

(fn `key_char_lower_v`
  (`self.Key Base` "/Game/HUI/BP/common/char_BP/char/lower/char_lower_v_BP.char_lower_v_BP_C"))

(fn `key_char_lower_w`
  (`self.Key Base` "/Game/HUI/BP/common/char_BP/char/lower/char_lower_w_BP.char_lower_w_BP_C"))

(fn `key_char_lower_x`
  (`self.Key Base` "/Game/HUI/BP/common/char_BP/char/lower/char_lower_x_BP.char_lower_x_BP_C"))

(fn `key_char_lower_y`
  (`self.Key Base` "/Game/HUI/BP/common/char_BP/char/lower/char_lower_y_BP.char_lower_y_BP_C"))

(fn `key_char_lower_z`
  (`self.Key Base` "/Game/HUI/BP/common/char_BP/char/lower/char_lower_z_BP.char_lower_z_BP_C"))

(fn `key_char_upper_A`
  (`self.Key Base` "/Game/HUI/BP/common/char_BP/char/upper/char_A_BP.char_A_BP_C"))

(fn `key_char_upper_B`
  (`self.Key Base` "/Game/HUI/BP/common/char_BP/char/upper/char_N_BP.char_N_BP_C"))

(fn `key_char_upper_C`
  (`self.Key Base` "/Game/HUI/BP/common/char_BP/char/upper/char_C_BP.char_C_BP_C"))

(fn `key_char_upper_D`
  (`self.Key Base` "/Game/HUI/BP/common/char_BP/char/upper/char_D_BP.char_D_BP_C"))

(fn `key_char_upper_E`
  (`self.Key Base` "/Game/HUI/BP/common/char_BP/char/upper/char_E_BP.char_E_BP_C"))

(fn `key_char_upper_F`
  (`self.Key Base` "/Game/HUI/BP/common/char_BP/char/upper/char_F_BP.char_F_BP_C"))

(fn `key_char_upper_G`
  (`self.Key Base` "/Game/HUI/BP/common/char_BP/char/upper/char_G_BP.char_G_BP_C"))

(fn `key_char_upper_H`
  (`self.Key Base` "/Game/HUI/BP/common/char_BP/char/upper/char_H_BP.char_H_BP_C"))

(fn `key_char_upper_I`
  (`self.Key Base` "/Game/HUI/BP/common/char_BP/char/upper/char_I_BP.char_I_BP_C"))

(fn `key_char_upper_J`
  (`self.Key Base` "/Game/HUI/BP/common/char_BP/char/upper/char_J_BP.char_J_BP_C"))

(fn `key_char_upper_K`
  (`self.Key Base` "/Game/HUI/BP/common/char_BP/char/upper/char_K_BP.char_K_BP_C"))

(fn `key_char_upper_L`
  (`self.Key Base` "/Game/HUI/BP/common/char_BP/char/upper/char_L_BP.char_L_BP_C"))

(fn `key_char_upper_M`
  (`self.Key Base` "/Game/HUI/BP/common/char_BP/char/upper/char_M_BP.char_M_BP_C"))

(fn `key_char_upper_N`
  (`self.Key Base` "/Game/HUI/BP/common/char_BP/char/upper/char_N_BP.char_N_BP_C"))

(fn `key_char_upper_O`
  (`self.Key Base` "/Game/HUI/BP/common/char_BP/char/upper/char_O_BP.char_O_BP_C"))

(fn `key_char_upper_P`
  (`self.Key Base` "/Game/HUI/BP/common/char_BP/char/upper/char_P_BP.char_P_BP_C"))

(fn `key_char_upper_Q`
  (`self.Key Base` "/Game/HUI/BP/common/char_BP/char/upper/char_Q_BP.char_Q_BP_C"))

(fn `key_char_upper_R`
  (`self.Key Base` "/Game/HUI/BP/common/char_BP/char/upper/char_R_BP.char_R_BP_C"))

(fn `key_char_upper_S`
  (`self.Key Base` "/Game/HUI/BP/common/char_BP/char/upper/char_S_BP.char_S_BP_C"))

(fn `key_char_upper_T`
  (`self.Key Base` "/Game/HUI/BP/common/char_BP/char/upper/char_T_BP.char_T_BP_C"))

(fn `key_char_upper_U`
  (`self.Key Base` "/Game/HUI/BP/common/char_BP/char/upper/char_U_BP.char_U_BP_C"))

(fn `key_char_upper_V`
  (`self.Key Base` "/Game/HUI/BP/common/char_BP/char/upper/char_V_BP.char_V_BP_C"))

(fn `key_char_upper_W`
  (`self.Key Base` "/Game/HUI/BP/common/char_BP/char/upper/char_W_BP.char_W_BP_C"))

(fn `key_char_upper_X`
  (`self.Key Base` "/Game/HUI/BP/common/char_BP/char/upper/char_X_BP.char_X_BP_C"))

(fn `key_char_upper_Y`
  (`self.Key Base` "/Game/HUI/BP/common/char_BP/char/upper/char_Y_BP.char_Y_BP_C"))

(fn `key_char_upper_Z`
  (`self.Key Base` "/Game/HUI/BP/common/char_BP/char/upper/char_Z_BP.char_Z_BP_C"))

(fn `key_number_0`
  (`self.Key Base` "/Game/HUI/BP/common/char_BP/number/number_0_BP.number_0_BP_C"))

(fn `key_number_1`
  (`self.Key Base` "/Game/HUI/BP/common/char_BP/number/number_1_BP.number_1_BP_C"))

(fn `key_number_2`
  (`self.Key Base` "/Game/HUI/BP/common/char_BP/number/number_2_BP.number_2_BP_C"))

(fn `key_number_3`
  (`self.Key Base` "/Game/HUI/BP/common/char_BP/number/number_3_BP.number_3_BP_C"))

(fn `key_number_4`
  (`self.Key Base` "/Game/HUI/BP/common/char_BP/number/number_4_BP.number_4_BP_C"))

(fn `key_number_5`
  (`self.Key Base` "/Game/HUI/BP/common/char_BP/number/number_5_BP.number_5_BP_C"))

(fn `key_number_6`
  (`self.Key Base` "/Game/HUI/BP/common/char_BP/number/number_6_BP.number_6_BP_C"))

(fn `key_number_7`
  (`self.Key Base` "/Game/HUI/BP/common/char_BP/number/number_7_BP.number_7_BP_C"))

(fn `key_number_8`
  (`self.Key Base` "/Game/HUI/BP/common/char_BP/number/number_8_BP.number_8_BP_C"))

(fn `key_number_9`
  (`self.Key Base` "/Game/HUI/BP/common/char_BP/number/number_9_BP.number_9_BP_C"))

(fn `key_symbol_ampersand`
  (`self.Key Base` "/Game/HUI/BP/common/char_BP/symbol/symbol_ampersand_BP.symbol_ampersand_BP_C"))

(fn `key_symbol_at`
  (`self.Key Base` "/Game/HUI/BP/common/char_BP/symbol/symbol_at_BP.symbol_at_BP_C"))

(fn `key_symbol_backquote`
  (`self.Key Base` "/Game/HUI/BP/common/char_BP/symbol/symbol_backquote_BP.symbol_backquote_BP_C"))

(fn `key_symbol_backslash`
  (`self.Key Base` "/Game/HUI/BP/common/char_BP/symbol/symbol_backslash_BP.symbol_backslash_BP_C"))

(fn `key_symbol_backspace`
  (locals (char_base_bp_temp :type "/Game/HUI/BP/common/char_BP/base/char_base_BP Object Reference"))
  (bind _cursor (`self.cursor`))
  (bind _char_list (`self.char_list`))
  (bind _char_list_2 (`self.char_list`))
  (bind (_relativelocation_x _relativelocation_y _relativelocation_z) (`KismetMathLibrary.BreakVector` (`SceneComponent.RelativeLocation` _cursor)))
  (bind _relativelocation_x_2 (`KismetMathLibrary.BreakVector` (`SceneComponent.RelativeLocation` (`/Game/HUI/BP/common/char_BP/base/char_base_BP.DefaultSceneRoot` (`local.char_base_bp_temp`)))))
  (bind _output (`|GetArrayItem` _char_list_2 (- (`KismetArrayLibrary.Array_Length` _char_list_2) 1)))
  (if (>= (`KismetArrayLibrary.Array_Length` (`self.char_list`)) 1)
    (`|ExecutionSequence`
      (:`then_0`
        ;[1 1 1] char base transform
        ;;[1 1 1] transform temp
        (set `self.curcor_transform_temp` (`SceneComponent.GetRelativeTransform` (`/Game/HUI/BP/common/char_BP/base/char_base_BP.DefaultSceneRoot` (`|GetArrayItem` _char_list (- (`KismetArrayLibrary.Array_Length` _char_list) 1))))))
      (:`then_1`
        ;[1 1 1] remove from list
        (set `local.char_base_bp_temp` _output)
        (`KismetArrayLibrary.Array_RemoveItem` _char_list_2 _output))
      (:`then_2`
        ;[1 1 1] set sursor relative location
        (`SceneComponent.K2_SetRelativeLocation` _cursor (`KismetMathLibrary.MakeVector` _relativelocation_x_2 _relativelocation_y _relativelocation_z) false false)
        ;[1 1 1] set visibility of cursor
        (if (not (`SceneComponent.bVisible` (`self.cursor`)))
          (`SceneComponent.SetVisibility` (`self.cursor`) true false)
          ;[1 1 1] set end_object to available
          (bind _asend_object (cast `/Game/HUI/BP/common/component/input/base/end_object` (`ChildActorComponent.ChildActor` (`self.end_object`))))
          (`/Game/HUI/BP/common/component/input/base/end_object.material_for_available` _asend_object)))
      (:`then_3`
        ;[1 1 1] destroy
        (`self.K2_DestroyActor` (`local.char_base_bp_temp`))))))

(fn `key_symbol_bar`
  (`self.Key Base` "/Game/HUI/BP/common/char_BP/symbol/symbol_bar_BP.symbol_bar_BP_C"))

(fn `key_symbol_braceleft`
  (`self.Key Base` "/Game/HUI/BP/common/char_BP/symbol/symbol_braceleft_BP.symbol_braceleft_BP_C"))

(fn `key_symbol_braceright`
  (`self.Key Base` "/Game/HUI/BP/common/char_BP/symbol/symbol_braceright_BP.symbol_braceright_BP_C"))

(fn `key_symbol_bracketleft`
  (`self.Key Base` "/Game/HUI/BP/common/char_BP/symbol/symbol_bracketleft_BP.symbol_bracketleft_BP_C"))

(fn `key_symbol_bracketright`
  (`self.Key Base` "/Game/HUI/BP/common/char_BP/symbol/symbol_bracketright_BP.symbol_bracketright_BP_C"))

(fn `key_symbol_caret`
  (`self.Key Base` "/Game/HUI/BP/common/char_BP/symbol/symbol_caret_BP.symbol_caret_BP_C"))

(fn `key_symbol_colon`
  (`self.Key Base` "/Game/HUI/BP/common/char_BP/symbol/symbol_colon_BP.symbol_colon_BP_C"))

(fn `key_symbol_comma`
  (`self.Key Base` "/Game/HUI/BP/common/char_BP/symbol/symbol_comma_BP.symbol_comma_BP_C"))

(fn `key_symbol_dollar`
  (`self.Key Base` "/Game/HUI/BP/common/char_BP/symbol/symbol_dollar_BP.symbol_dollar_BP_C"))

(fn `key_symbol_dot`
  (`self.Key Base` "/Game/HUI/BP/common/char_BP/symbol/symbol_dot_BP.symbol_dot_BP_C"))

(fn `key_symbol_doublequote`
  (`self.Key Base` "/Game/HUI/BP/common/char_BP/symbol/symbol_doublequote_BP.symbol_doublequote_BP_C"))

(fn `key_symbol_equal`
  (`self.Key Base` "/Game/HUI/BP/common/char_BP/symbol/symbol_equal_BP.symbol_equal_BP_C"))

(fn `key_symbol_exlcam`
  (`self.Key Base` "/Game/HUI/BP/common/char_BP/symbol/symbol_exclam_BP.symbol_exclam_BP_C"))

(fn `key_symbol_greater`
  (`self.Key Base` "/Game/HUI/BP/common/char_BP/symbol/symbol_greater_BP.symbol_greater_BP_C"))

(fn `key_symbol_hyphen`
  (`self.Key Base` "/Game/HUI/BP/common/char_BP/symbol/symbol_hyphen_BP.symbol_hyphen_BP_C"))

(fn `key_symbol_less`
  (`self.Key Base` "/Game/HUI/BP/common/char_BP/symbol/symbol_less_BP.symbol_less_BP_C"))

(fn `key_symbol_minus`
  (`self.Key Base` "/Game/HUI/BP/common/char_BP/symbol/symbol_minus_BP.symbol_minus_BP_C"))

(fn `key_symbol_numbersign`
  (`self.Key Base` "/Game/HUI/BP/common/char_BP/symbol/symbol_numbersign_BP.symbol_numbersign_BP_C"))

(fn `key_symbol_parenleft`
  (`self.Key Base` "/Game/HUI/BP/common/char_BP/symbol/symbol_parenleft_BP.symbol_parenleft_BP_C"))

(fn `key_symbol_parenright`
  (`self.Key Base` "/Game/HUI/BP/common/char_BP/symbol/symbol_parenright_BP.symbol_parenright_BP_C"))

(fn `key_symbol_percent`
  (`self.Key Base` "/Game/HUI/BP/common/char_BP/symbol/symbol_percent_BP.symbol_percent_BP_C"))

(fn `key_symbol_plus`
  (`self.Key Base` "/Game/HUI/BP/common/char_BP/symbol/symbol_plus_BP.symbol_plus_BP_C"))

(fn `key_symbol_questionmark`
  (`self.Key Base` "/Game/HUI/BP/common/char_BP/symbol/symbol_questionmark_BP.symbol_questionmark_BP_C"))

(fn `key_symbol_quote`
  (`self.Key Base` "/Game/HUI/BP/common/char_BP/symbol/symbol_quote_BP.symbol_quote_BP_C"))

(fn `key_symbol_semicolon`
  (`self.Key Base` "/Game/HUI/BP/common/char_BP/symbol/symbol_semicolon_BP.symbol_semicolon_BP_C"))

(fn `key_symbol_slash`
  (`self.Key Base` "/Game/HUI/BP/common/char_BP/symbol/symbol_slash_BP.symbol_slash_BP_C"))

(fn `key_symbol_space_bar`)

(fn `key_symbol_star`
  (`self.Key Base` "/Game/HUI/BP/common/char_BP/symbol/symbol_star_BP.symbol_star_BP_C"))

(fn `key_symbol_tilde`
  (`self.Key Base` "/Game/HUI/BP/common/char_BP/symbol/symbol_tilde_BP.symbol_tilde_BP_C"))

(fn `set_input_body_material`
  (params (material :type "Material Object Reference") (`emissive color densy` :type "Float (double-precision)"))
  (bind _input_body (`self.input_body`))
  (`/Engine/EditorBlueprintResources/StandardMacros.IsValid` material
    (:`Is Valid`
      (`PrimitiveComponent.SetMaterial` _input_body 0 material))
    (:`Is Not Valid`
      _))
  (`MeshComponent.SetScalarParameterValueOnMaterials` _input_body (`self.emissive color densy name`) `emissive color densy`))

(fn `set_input_border_material`
  (params (material :type "Material Object Reference") (`emissive color densy` :type "Float (double-precision)"))
  (bind _input_border (`self.input_border`))
  (`/Engine/EditorBlueprintResources/StandardMacros.IsValid` material
    (:`Is Valid`
      (`PrimitiveComponent.SetMaterial` _input_border 0 material))
    (:`Is Not Valid`
      _))
  (`MeshComponent.SetScalarParameterValueOnMaterials` _input_border (`self.emissive color densy name`) `emissive color densy`))

(fn `UserConstructionScript`)