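; Cursor Blueprint in the common input component set that blinks its CursorBody.
; On BeginPlay a looping half-second timer fires the flash event, which calls FlashFunction.
; Each call toggles the IsFlash flag, switching both the body's visibility and an emissive density material parameter between off and bright.
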(event `self.ReceiveBeginPlay`
  (`KismetSystemLibrary.K2_SetTimerDelegate` (delegate `flash`) 0.5 true))

(event `flash`
  (`self.flash_function`))

(fn `flash_function`
  (if (`self.is_flash`)
    (`MeshComponent.SetScalarParameterValueOnMaterials` (`self.cursor_body`) (`self.emissive color densy name`) 0.0)
    (set `self.is_flash` false)
    (`SceneComponent.SetVisibility` (`self.cursor_body`) false false)
    (else
      (`MeshComponent.SetScalarParameterValueOnMaterials` (`self.cursor_body`) (`self.emissive color densy name`) 100.0)
      (set `self.is_flash` true)
      (`SceneComponent.SetVisibility` (`self.cursor_body`) true false))))

(fn `UserConstructionScript`)