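; Base Blueprint for a clickable 3D button with a glowing body, border and text label.
; BeginPlay sets emissive strength on button and border, then spawns a TextBP actor at an offset transform to render InputString as left-aligned 3D text.
; Clicking Onclick_cube sinks the button and swaps in a highlight material, restoring both after a short delay.
; An IsClicking flag blocks re-clicks meanwhile; the click triggers only visual feedback here.
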(event `self.ReceiveBeginPlay`
  (bind _returnvalue (`SceneComponent.K2_GetComponentToWorld` (`self.DefaultSceneRoot`)))
  (`|ExecutionSequence`
    (:`then_0`
      (`self.init_function`))
    (:`then_1`
      ;[1 1 1] show button text
      (bind _returnvalue_2 (`|SpawnActorFromClass` (`self.text_BP`) (`KismetMathLibrary.MakeTransform` (`KismetMathLibrary.MakeVector` (+ (.x (.location _returnvalue)) (`self.location_x_offset`)) (+ (.y (.location _returnvalue)) (`self.location_y_offset`)) (+ (.z (.location _returnvalue)) (`self.location_z_offset`))) (.rotation _returnvalue) (`KismetMathLibrary.MakeVector` (* (.x (.scale _returnvalue)) (`self.scale_x_offset`)) (* (.y (.scale _returnvalue)) (`self.scale_y_offset`)) (* (.z (.scale _returnvalue)) (`self.scale_z_offset`)))) "Undefined" "OverrideRootScale" null null))
      (bind _output_get (set `self.text_BP_temp` _returnvalue_2))
      (set `/Game/BP/common/component/text/text_base_BP.char_material` (`self.Char Meterial`) _output_get)
      (`self.Show Button 3D text`))))

(event `self.onclick_cube.OnClicked`
  (params (TouchedComponent :type "PrimitiveComponent Object Reference") (ButtonPressed :type "Key Structure"))
  ;[1 1 1] button on click
  (if (not (`self.is_clicking`))
    (set `self.is_clicking` true)
    (`self.Onclick Function`)
    (`KismetSystemLibrary.Delay` 0.2)
    (`self.onreleased_function`)
    (set `self.is_clicking` false)))

(fn `init_function`
  (`self.set_button_material` null (`self.button Emissive Color Densy`))
  (`self.set_button_border_material` null (`self.button_border Emissive Color Densy`)))

(fn `Onclick Function`
  (bind _button (`self.button`))
  (bind (_relativelocation_x _relativelocation_y _relativelocation_z) (`KismetMathLibrary.BreakVector` (`SceneComponent.RelativeLocation` _button)))
  (set `self.onclick_origin_material_temp` (`PrimitiveComponent.GetMaterial` _button 0))
  (`SceneComponent.K2_SetRelativeLocation` _button (`KismetMathLibrary.MakeVector` _relativelocation_x _relativelocation_y (- _relativelocation_z 8.0)) false false)
  (`PrimitiveComponent.SetMaterial` _button 0 (`self.onclick Meterial`))
  (`MeshComponent.SetScalarParameterValueOnMaterials` _button (`self.Emissive Color Densy`) (`self.onclick Emissive Color Densy`)))

(fn `onreleased_function`
  (bind _button (`self.button`))
  (bind (_relativelocation_x _relativelocation_y _relativelocation_z) (`KismetMathLibrary.BreakVector` (`SceneComponent.RelativeLocation` _button)))
  (`SceneComponent.K2_SetRelativeLocation` _button (`KismetMathLibrary.MakeVector` _relativelocation_x _relativelocation_y (+ _relativelocation_z 8.0)) false false)
  (`PrimitiveComponent.SetMaterial` _button 0 (`self.onclick_origin_material_temp`))
  (`MeshComponent.SetScalarParameterValueOnMaterials` _button (`self.Emissive Color Densy`) (`self.button Emissive Color Densy`)))

(fn `set_button_border_material`
  (params (button_border_material :type "Material Object Reference") (`Emissive Color Densy` :type "Float (double-precision)"))
  (bind _button_border (`self.button_border`))
  (`/Engine/EditorBlueprintResources/StandardMacros.IsValid` button_border_material
    (:`Is Valid`
      (`PrimitiveComponent.SetMaterial` _button_border 0 button_border_material))
    (:`Is Not Valid`
      _))
  (`MeshComponent.SetScalarParameterValueOnMaterials` _button_border (`self.Emissive Color Densy`) `Emissive Color Densy`))

(fn `set_button_material`
  (params (button_material :type "Material Object Reference") (`button Emissive Color Densy` :type "Float (double-precision)"))
  (bind _button (`self.button`))
  (`/Engine/EditorBlueprintResources/StandardMacros.IsValid` button_material
    (:`Is Valid`
      (`PrimitiveComponent.SetMaterial` _button 0 button_material))
    (:`Is Not Valid`
      _))
  (`MeshComponent.SetScalarParameterValueOnMaterials` _button (`self.Emissive Color Densy`) `button Emissive Color Densy`))

(fn `Show Button 3D text`
  (bind _text_bp_temp (`self.text_BP_temp`))
  (set `/Game/BP/common/component/text/text_base_BP.input_string` (`self.input_string`) _text_bp_temp)
  (`/Game/BP/common/component/text/text_base_BP.Show _3D_String_left_layout` _text_bp_temp (`self.input_text Emissive Color Densy`) (`self.Char Meterial`)))

(fn `UserConstructionScript`)