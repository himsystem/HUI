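; Base player controller that turns raw keyboard presses into per-character input events for letters, digits, symbols, space and backspace.
; Each key or Shift combination calls its matching function on InputEventBaseBPTemp after a validity check, and Shift+F fires on release as well as press.
; BeginPlay calls InitFunction, which is empty here, and nothing in this Blueprint assigns the receiver.
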(event `self.ReceiveBeginPlay`
  (`self.init_function`))

(event `Key|Shift+Q`
  (params (Key :type "Key Structure"))
  (bind _input_event_base_bp_temp (`self.input_event_base_BP_temp`))
  ;[1 1 1] char upper case
  (:`Pressed`
    (`/Engine/EditorBlueprintResources/StandardMacros.IsValid` _input_event_base_bp_temp
      (:`Is Valid`
        (`/Game/BP/common/component/input/base/input_event_base_BP.key_char_upper_Q` _input_event_base_bp_temp)))))

(event `Key|Q`
  (params (Key :type "Key Structure"))
  (bind _input_event_base_bp_temp (`self.input_event_base_BP_temp`))
  ;[1 1 1] char lower case
  (:`Pressed`
    (`/Engine/EditorBlueprintResources/StandardMacros.IsValid` _input_event_base_bp_temp
      (:`Is Valid`
        (`/Game/BP/common/component/input/base/input_event_base_BP.key_char_lower_q` _input_event_base_bp_temp)))))

(event `Key|Zero`
  (params (Key :type "Key Structure"))
  (bind _input_event_base_bp_temp (`self.input_event_base_BP_temp`))
  ;[1 1 1] number
  (:`Pressed`
    (`/Engine/EditorBlueprintResources/StandardMacros.IsValid` _input_event_base_bp_temp
      (:`Is Valid`
        (`/Game/BP/common/component/input/base/input_event_base_BP.key_number_0` _input_event_base_bp_temp)))))

(event `Key|Tilde`
  (params (Key :type "Key Structure"))
  (bind _input_event_base_bp_temp (`self.input_event_base_BP_temp`))
  ;[1 1 1] symbol
  (:`Pressed`
    (`/Engine/EditorBlueprintResources/StandardMacros.IsValid` _input_event_base_bp_temp
      (:`Is Valid`
        (`/Game/BP/common/component/input/base/input_event_base_BP.key_symbol_backquote` _input_event_base_bp_temp)))))

(event `Key|One`
  (params (Key :type "Key Structure"))
  (bind _input_event_base_bp_temp (`self.input_event_base_BP_temp`))
  ;[1 1 1] number
  (:`Pressed`
    (`/Engine/EditorBlueprintResources/StandardMacros.IsValid` _input_event_base_bp_temp
      (:`Is Valid`
        (`/Game/BP/common/component/input/base/input_event_base_BP.key_number_1` _input_event_base_bp_temp)))))

(event `Key|Shift+W`
  (params (Key :type "Key Structure"))
  (bind _input_event_base_bp_temp (`self.input_event_base_BP_temp`))
  ;[1 1 1] char upper case
  (:`Pressed`
    (`/Engine/EditorBlueprintResources/StandardMacros.IsValid` _input_event_base_bp_temp
      (:`Is Valid`
        (`/Game/BP/common/component/input/base/input_event_base_BP.key_char_upper_W` _input_event_base_bp_temp)))))

(event `Key|W`
  (params (Key :type "Key Structure"))
  (bind _input_event_base_bp_temp (`self.input_event_base_BP_temp`))
  ;[1 1 1] char lower case
  (:`Pressed`
    (`/Engine/EditorBlueprintResources/StandardMacros.IsValid` _input_event_base_bp_temp
      (:`Is Valid`
        (`/Game/BP/common/component/input/base/input_event_base_BP.key_char_lower_w` _input_event_base_bp_temp)))))

(event `Key|Shift+Tilde`
  (params (Key :type "Key Structure"))
  (bind _input_event_base_bp_temp (`self.input_event_base_BP_temp`))
  ;[1 1 1] symbol
  (:`Pressed`
    (`/Engine/EditorBlueprintResources/StandardMacros.IsValid` _input_event_base_bp_temp
      (:`Is Valid`
        (`/Game/BP/common/component/input/base/input_event_base_BP.key_symbol_tilde` _input_event_base_bp_temp)))))

(event `Key|Shift+E`
  (params (Key :type "Key Structure"))
  (bind _input_event_base_bp_temp (`self.input_event_base_BP_temp`))
  ;[1 1 1] char upper case
  (:`Pressed`
    (`/Engine/EditorBlueprintResources/StandardMacros.IsValid` _input_event_base_bp_temp
      (:`Is Valid`
        (`/Game/BP/common/component/input/base/input_event_base_BP.key_char_upper_E` _input_event_base_bp_temp)))))

(event `Key|E`
  (params (Key :type "Key Structure"))
  (bind _input_event_base_bp_temp (`self.input_event_base_BP_temp`))
  ;[1 1 1] char lower case
  (:`Pressed`
    (`/Engine/EditorBlueprintResources/StandardMacros.IsValid` _input_event_base_bp_temp
      (:`Is Valid`
        (`/Game/BP/common/component/input/base/input_event_base_BP.key_char_lower_e` _input_event_base_bp_temp)))))

(event `Key|Two`
  (params (Key :type "Key Structure"))
  (bind _input_event_base_bp_temp (`self.input_event_base_BP_temp`))
  ;[1 1 1] number
  (:`Pressed`
    (`/Engine/EditorBlueprintResources/StandardMacros.IsValid` _input_event_base_bp_temp
      (:`Is Valid`
        (`/Game/BP/common/component/input/base/input_event_base_BP.key_number_2` _input_event_base_bp_temp)))))

(event `Key|Shift+One`
  (params (Key :type "Key Structure"))
  (bind _input_event_base_bp_temp (`self.input_event_base_BP_temp`))
  ;[1 1 1] symbol
  (:`Pressed`
    (`/Engine/EditorBlueprintResources/StandardMacros.IsValid` _input_event_base_bp_temp
      (:`Is Valid`
        (`/Game/BP/common/component/input/base/input_event_base_BP.key_symbol_exlcam` _input_event_base_bp_temp)))))

(event `Key|Shift+R`
  (params (Key :type "Key Structure"))
  (bind _input_event_base_bp_temp (`self.input_event_base_BP_temp`))
  ;[1 1 1] char upper case
  (:`Pressed`
    (`/Engine/EditorBlueprintResources/StandardMacros.IsValid` _input_event_base_bp_temp
      (:`Is Valid`
        (`/Game/BP/common/component/input/base/input_event_base_BP.key_char_upper_R` _input_event_base_bp_temp)))))

(event `Key|R`
  (params (Key :type "Key Structure"))
  (bind _input_event_base_bp_temp (`self.input_event_base_BP_temp`))
  ;[1 1 1] char lower case
  (:`Pressed`
    (`/Engine/EditorBlueprintResources/StandardMacros.IsValid` _input_event_base_bp_temp
      (:`Is Valid`
        (`/Game/BP/common/component/input/base/input_event_base_BP.key_char_lower_r` _input_event_base_bp_temp)))))

(event `Key|Shift+Two`
  (params (Key :type "Key Structure"))
  (bind _input_event_base_bp_temp (`self.input_event_base_BP_temp`))
  ;[1 1 1] symbol
  (:`Pressed`
    (`/Engine/EditorBlueprintResources/StandardMacros.IsValid` _input_event_base_bp_temp
      (:`Is Valid`
        (`/Game/BP/common/component/input/base/input_event_base_BP.key_symbol_at` _input_event_base_bp_temp)))))

(event `Key|Three`
  (params (Key :type "Key Structure"))
  (bind _input_event_base_bp_temp (`self.input_event_base_BP_temp`))
  ;[1 1 1] number
  (:`Pressed`
    (`/Engine/EditorBlueprintResources/StandardMacros.IsValid` _input_event_base_bp_temp
      (:`Is Valid`
        (`/Game/BP/common/component/input/base/input_event_base_BP.key_number_3` _input_event_base_bp_temp)))))

(event `Key|Shift+T`
  (params (Key :type "Key Structure"))
  (bind _input_event_base_bp_temp (`self.input_event_base_BP_temp`))
  ;[1 1 1] char upper case
  (:`Pressed`
    (`/Engine/EditorBlueprintResources/StandardMacros.IsValid` _input_event_base_bp_temp
      (:`Is Valid`
        (`/Game/BP/common/component/input/base/input_event_base_BP.key_char_upper_T` _input_event_base_bp_temp)))))

(event `Key|Shift+Three`
  (params (Key :type "Key Structure"))
  (bind _input_event_base_bp_temp (`self.input_event_base_BP_temp`))
  ;[1 1 1] symbol
  (:`Pressed`
    (`/Engine/EditorBlueprintResources/StandardMacros.IsValid` _input_event_base_bp_temp
      (:`Is Valid`
        (`/Game/BP/common/component/input/base/input_event_base_BP.key_symbol_numbersign` _input_event_base_bp_temp)))))

(event `Key|T`
  (params (Key :type "Key Structure"))
  (bind _input_event_base_bp_temp (`self.input_event_base_BP_temp`))
  ;[1 1 1] char lower case
  (:`Pressed`
    (`/Engine/EditorBlueprintResources/StandardMacros.IsValid` _input_event_base_bp_temp
      (:`Is Valid`
        (`/Game/BP/common/component/input/base/input_event_base_BP.key_char_lower_t` _input_event_base_bp_temp)))))

(event `Key|Four`
  (params (Key :type "Key Structure"))
  (bind _input_event_base_bp_temp (`self.input_event_base_BP_temp`))
  ;[1 1 1] number
  (:`Pressed`
    (`/Engine/EditorBlueprintResources/StandardMacros.IsValid` _input_event_base_bp_temp
      (:`Is Valid`
        (`/Game/BP/common/component/input/base/input_event_base_BP.key_number_4` _input_event_base_bp_temp)))))

(event `Key|Shift+Four`
  (params (Key :type "Key Structure"))
  (bind _input_event_base_bp_temp (`self.input_event_base_BP_temp`))
  ;[1 1 1] symbol
  (:`Pressed`
    (`/Engine/EditorBlueprintResources/StandardMacros.IsValid` _input_event_base_bp_temp
      (:`Is Valid`
        (`/Game/BP/common/component/input/base/input_event_base_BP.key_symbol_dollar` _input_event_base_bp_temp)))))

(event `Key|Shift+Y`
  (params (Key :type "Key Structure"))
  (bind _input_event_base_bp_temp (`self.input_event_base_BP_temp`))
  ;[1 1 1] char upper case
  (:`Pressed`
    (`/Engine/EditorBlueprintResources/StandardMacros.IsValid` _input_event_base_bp_temp
      (:`Is Valid`
        (`/Game/BP/common/component/input/base/input_event_base_BP.key_char_upper_Y` _input_event_base_bp_temp)))))

(event `Key|Y`
  (params (Key :type "Key Structure"))
  (bind _input_event_base_bp_temp (`self.input_event_base_BP_temp`))
  ;[1 1 1] char lower case
  (:`Pressed`
    (`/Engine/EditorBlueprintResources/StandardMacros.IsValid` _input_event_base_bp_temp
      (:`Is Valid`
        (`/Game/BP/common/component/input/base/input_event_base_BP.key_char_lower_y` _input_event_base_bp_temp)))))

(event `Key|Shift+Five`
  (params (Key :type "Key Structure"))
  (bind _input_event_base_bp_temp (`self.input_event_base_BP_temp`))
  ;[1 1 1] symbol
  (:`Pressed`
    (`/Engine/EditorBlueprintResources/StandardMacros.IsValid` _input_event_base_bp_temp
      (:`Is Valid`
        (`/Game/BP/common/component/input/base/input_event_base_BP.key_symbol_percent` _input_event_base_bp_temp)))))

(event `Key|Five`
  (params (Key :type "Key Structure"))
  (bind _input_event_base_bp_temp (`self.input_event_base_BP_temp`))
  ;[1 1 1] number
  (:`Pressed`
    (`/Engine/EditorBlueprintResources/StandardMacros.IsValid` _input_event_base_bp_temp
      (:`Is Valid`
        (`/Game/BP/common/component/input/base/input_event_base_BP.key_number_5` _input_event_base_bp_temp)))))

(event `Key|Shift+U`
  (params (Key :type "Key Structure"))
  (bind _input_event_base_bp_temp (`self.input_event_base_BP_temp`))
  ;[1 1 1] char upper case
  (:`Pressed`
    (`/Engine/EditorBlueprintResources/StandardMacros.IsValid` _input_event_base_bp_temp
      (:`Is Valid`
        (`/Game/BP/common/component/input/base/input_event_base_BP.key_char_upper_U` _input_event_base_bp_temp)))))

(event `Key|U`
  (params (Key :type "Key Structure"))
  (bind _input_event_base_bp_temp (`self.input_event_base_BP_temp`))
  ;[1 1 1] char lower case
  (:`Pressed`
    (`/Engine/EditorBlueprintResources/StandardMacros.IsValid` _input_event_base_bp_temp
      (:`Is Valid`
        (`/Game/BP/common/component/input/base/input_event_base_BP.key_char_lower_u` _input_event_base_bp_temp)))))

(event `Key|Shift+Six`
  (params (Key :type "Key Structure"))
  (bind _input_event_base_bp_temp (`self.input_event_base_BP_temp`))
  ;[1 1 1] symbol
  (:`Pressed`
    (`/Engine/EditorBlueprintResources/StandardMacros.IsValid` _input_event_base_bp_temp
      (:`Is Valid`
        (`/Game/BP/common/component/input/base/input_event_base_BP.key_symbol_caret` _input_event_base_bp_temp)))))

(event `Key|Six`
  (params (Key :type "Key Structure"))
  (bind _input_event_base_bp_temp (`self.input_event_base_BP_temp`))
  ;[1 1 1] number
  (:`Pressed`
    (`/Engine/EditorBlueprintResources/StandardMacros.IsValid` _input_event_base_bp_temp
      (:`Is Valid`
        (`/Game/BP/common/component/input/base/input_event_base_BP.key_number_6` _input_event_base_bp_temp)))))

(event `Key|Shift+I`
  (params (Key :type "Key Structure"))
  (bind _input_event_base_bp_temp (`self.input_event_base_BP_temp`))
  ;[1 1 1] char upper case
  (:`Pressed`
    (`/Engine/EditorBlueprintResources/StandardMacros.IsValid` _input_event_base_bp_temp
      (:`Is Valid`
        (`/Game/BP/common/component/input/base/input_event_base_BP.key_char_upper_I` _input_event_base_bp_temp)))))

(event `Key|I`
  (params (Key :type "Key Structure"))
  (bind _input_event_base_bp_temp (`self.input_event_base_BP_temp`))
  ;[1 1 1] char lower case
  (:`Pressed`
    (`/Engine/EditorBlueprintResources/StandardMacros.IsValid` _input_event_base_bp_temp
      (:`Is Valid`
        (`/Game/BP/common/component/input/base/input_event_base_BP.key_char_lower_i` _input_event_base_bp_temp)))))

(event `Key|Shift+Seven`
  (params (Key :type "Key Structure"))
  (bind _input_event_base_bp_temp (`self.input_event_base_BP_temp`))
  ;[1 1 1] symbol
  (:`Pressed`
    (`/Engine/EditorBlueprintResources/StandardMacros.IsValid` _input_event_base_bp_temp
      (:`Is Valid`
        (`/Game/BP/common/component/input/base/input_event_base_BP.key_symbol_ampersand` _input_event_base_bp_temp)))))

(event `Key|Seven`
  (params (Key :type "Key Structure"))
  (bind _input_event_base_bp_temp (`self.input_event_base_BP_temp`))
  ;[1 1 1] number
  (:`Pressed`
    (`/Engine/EditorBlueprintResources/StandardMacros.IsValid` _input_event_base_bp_temp
      (:`Is Valid`
        (`/Game/BP/common/component/input/base/input_event_base_BP.key_number_7` _input_event_base_bp_temp)))))

(event `Key|Shift+O`
  (params (Key :type "Key Structure"))
  (bind _input_event_base_bp_temp (`self.input_event_base_BP_temp`))
  ;[1 1 1] char upper case
  (:`Pressed`
    (`/Engine/EditorBlueprintResources/StandardMacros.IsValid` _input_event_base_bp_temp
      (:`Is Valid`
        (`/Game/BP/common/component/input/base/input_event_base_BP.key_char_upper_O` _input_event_base_bp_temp)))))

(event `Key|O`
  (params (Key :type "Key Structure"))
  (bind _input_event_base_bp_temp (`self.input_event_base_BP_temp`))
  ;[1 1 1] char lower case
  (:`Pressed`
    (`/Engine/EditorBlueprintResources/StandardMacros.IsValid` _input_event_base_bp_temp
      (:`Is Valid`
        (`/Game/BP/common/component/input/base/input_event_base_BP.key_char_lower_o` _input_event_base_bp_temp)))))

(event `Key|Shift+P`
  (params (Key :type "Key Structure"))
  (bind _input_event_base_bp_temp (`self.input_event_base_BP_temp`))
  ;[1 1 1] char upper case
  (:`Pressed`
    (`/Engine/EditorBlueprintResources/StandardMacros.IsValid` _input_event_base_bp_temp
      (:`Is Valid`
        (`/Game/BP/common/component/input/base/input_event_base_BP.key_char_upper_P` _input_event_base_bp_temp)))))

(event `Key|Shift+Eight`
  (params (Key :type "Key Structure"))
  (bind _input_event_base_bp_temp (`self.input_event_base_BP_temp`))
  ;[1 1 1] symbol
  (:`Pressed`
    (`/Engine/EditorBlueprintResources/StandardMacros.IsValid` _input_event_base_bp_temp
      (:`Is Valid`
        (`/Game/BP/common/component/input/base/input_event_base_BP.key_symbol_star` _input_event_base_bp_temp)))))

(event `Key|P`
  (params (Key :type "Key Structure"))
  (bind _input_event_base_bp_temp (`self.input_event_base_BP_temp`))
  ;[1 1 1] char lower case
  (:`Pressed`
    (`/Engine/EditorBlueprintResources/StandardMacros.IsValid` _input_event_base_bp_temp
      (:`Is Valid`
        (`/Game/BP/common/component/input/base/input_event_base_BP.key_char_lower_p` _input_event_base_bp_temp)))))

(event `Key|Eight`
  (params (Key :type "Key Structure"))
  (bind _input_event_base_bp_temp (`self.input_event_base_BP_temp`))
  ;[1 1 1] number
  (:`Pressed`
    (`/Engine/EditorBlueprintResources/StandardMacros.IsValid` _input_event_base_bp_temp
      (:`Is Valid`
        (`/Game/BP/common/component/input/base/input_event_base_BP.key_number_8` _input_event_base_bp_temp)))))

(event `Key|Shift+Nine`
  (params (Key :type "Key Structure"))
  (bind _input_event_base_bp_temp (`self.input_event_base_BP_temp`))
  ;[1 1 1] symbol
  (:`Pressed`
    (`/Engine/EditorBlueprintResources/StandardMacros.IsValid` _input_event_base_bp_temp
      (:`Is Valid`
        (`/Game/BP/common/component/input/base/input_event_base_BP.key_symbol_parenleft` _input_event_base_bp_temp)))))

(event `Key|Nine`
  (params (Key :type "Key Structure"))
  (bind _input_event_base_bp_temp (`self.input_event_base_BP_temp`))
  ;[1 1 1] number
  (:`Pressed`
    (`/Engine/EditorBlueprintResources/StandardMacros.IsValid` _input_event_base_bp_temp
      (:`Is Valid`
        (`/Game/BP/common/component/input/base/input_event_base_BP.key_number_9` _input_event_base_bp_temp)))))

(event `Key|Shift+A`
  (params (Key :type "Key Structure"))
  (bind _input_event_base_bp_temp (`self.input_event_base_BP_temp`))
  ;[1 1 1] char upper case
  (:`Pressed`
    (`/Engine/EditorBlueprintResources/StandardMacros.IsValid` _input_event_base_bp_temp
      (:`Is Valid`
        (`/Game/BP/common/component/input/base/input_event_base_BP.key_char_upper_A` _input_event_base_bp_temp)))))

(event `Key|A`
  (params (Key :type "Key Structure"))
  (bind _input_event_base_bp_temp (`self.input_event_base_BP_temp`))
  ;[1 1 1] char lower case
  (:`Pressed`
    (`/Engine/EditorBlueprintResources/StandardMacros.IsValid` _input_event_base_bp_temp
      (:`Is Valid`
        (`/Game/BP/common/component/input/base/input_event_base_BP.key_char_lower_a` _input_event_base_bp_temp)))))

(event `Key|Shift+Zero`
  (params (Key :type "Key Structure"))
  (bind _input_event_base_bp_temp (`self.input_event_base_BP_temp`))
  ;[1 1 1] symbol
  (:`Pressed`
    (`/Engine/EditorBlueprintResources/StandardMacros.IsValid` _input_event_base_bp_temp
      (:`Is Valid`
        (`/Game/BP/common/component/input/base/input_event_base_BP.key_symbol_parenright` _input_event_base_bp_temp)))))

(event `Key|Shift+S`
  (params (Key :type "Key Structure"))
  (bind _input_event_base_bp_temp (`self.input_event_base_BP_temp`))
  ;[1 1 1] char upper case
  (:`Pressed`
    (`/Engine/EditorBlueprintResources/StandardMacros.IsValid` _input_event_base_bp_temp
      (:`Is Valid`
        (`/Game/BP/common/component/input/base/input_event_base_BP.key_char_upper_S` _input_event_base_bp_temp)))))

(event `Key|S`
  (params (Key :type "Key Structure"))
  (bind _input_event_base_bp_temp (`self.input_event_base_BP_temp`))
  ;[1 1 1] char lower case
  (:`Pressed`
    (`/Engine/EditorBlueprintResources/StandardMacros.IsValid` _input_event_base_bp_temp
      (:`Is Valid`
        (`/Game/BP/common/component/input/base/input_event_base_BP.key_char_lower_s` _input_event_base_bp_temp)))))

(event `Key|Shift+Hyphen`
  (params (Key :type "Key Structure"))
  (bind _input_event_base_bp_temp (`self.input_event_base_BP_temp`))
  ;[1 1 1] symbol
  (:`Pressed`
    (`/Engine/EditorBlueprintResources/StandardMacros.IsValid` _input_event_base_bp_temp
      (:`Is Valid`
        (`/Game/BP/common/component/input/base/input_event_base_BP.key_symbol_minus` _input_event_base_bp_temp)))))

(event `Key|Shift+D`
  (params (Key :type "Key Structure"))
  (bind _input_event_base_bp_temp (`self.input_event_base_BP_temp`))
  ;[1 1 1] char upper case
  (:`Pressed`
    (`/Engine/EditorBlueprintResources/StandardMacros.IsValid` _input_event_base_bp_temp
      (:`Is Valid`
        (`/Game/BP/common/component/input/base/input_event_base_BP.key_char_upper_D` _input_event_base_bp_temp)))))

(event `Key|D`
  (params (Key :type "Key Structure"))
  (bind _input_event_base_bp_temp (`self.input_event_base_BP_temp`))
  ;[1 1 1] char lower case
  (:`Pressed`
    (`/Engine/EditorBlueprintResources/StandardMacros.IsValid` _input_event_base_bp_temp
      (:`Is Valid`
        (`/Game/BP/common/component/input/base/input_event_base_BP.key_char_lower_d` _input_event_base_bp_temp)))))

(event `Key|Shift+F`
  (params (Key :type "Key Structure"))
  (bind _input_event_base_bp_temp (`self.input_event_base_BP_temp`))
  ;[1 1 1] char upper case
  (:`Pressed`
    (`/Engine/EditorBlueprintResources/StandardMacros.IsValid` _input_event_base_bp_temp :!label _label
      (:`Is Valid`
        (`/Game/BP/common/component/input/base/input_event_base_BP.key_char_upper_F` _input_event_base_bp_temp))))
  (:`Released`
    (goto _label)))

(event `Key|F`
  (params (Key :type "Key Structure"))
  (bind _input_event_base_bp_temp (`self.input_event_base_BP_temp`))
  ;[1 1 1] char lower case
  (:`Pressed`
    (`/Engine/EditorBlueprintResources/StandardMacros.IsValid` _input_event_base_bp_temp
      (:`Is Valid`
        (`/Game/BP/common/component/input/base/input_event_base_BP.key_char_lower_f` _input_event_base_bp_temp)))))

(event `Key|Hyphen`
  (params (Key :type "Key Structure"))
  (bind _input_event_base_bp_temp (`self.input_event_base_BP_temp`))
  ;[1 1 1] symbol
  (:`Pressed`
    (`/Engine/EditorBlueprintResources/StandardMacros.IsValid` _input_event_base_bp_temp
      (:`Is Valid`
        (`/Game/BP/common/component/input/base/input_event_base_BP.key_symbol_hyphen` _input_event_base_bp_temp)))))

(event `Key|Shift+G`
  (params (Key :type "Key Structure"))
  (bind _input_event_base_bp_temp (`self.input_event_base_BP_temp`))
  ;[1 1 1] char upper case
  (:`Pressed`
    (`/Engine/EditorBlueprintResources/StandardMacros.IsValid` _input_event_base_bp_temp
      (:`Is Valid`
        (`/Game/BP/common/component/input/base/input_event_base_BP.key_char_upper_G` _input_event_base_bp_temp)))))

(event `Key|G`
  (params (Key :type "Key Structure"))
  (bind _input_event_base_bp_temp (`self.input_event_base_BP_temp`))
  ;[1 1 1] char lower case
  (:`Pressed`
    (`/Engine/EditorBlueprintResources/StandardMacros.IsValid` _input_event_base_bp_temp
      (:`Is Valid`
        (`/Game/BP/common/component/input/base/input_event_base_BP.key_char_lower_g` _input_event_base_bp_temp)))))

(event `Key|Equals`
  (params (Key :type "Key Structure"))
  (bind _input_event_base_bp_temp (`self.input_event_base_BP_temp`))
  ;[1 1 1] symbol
  (:`Pressed`
    (`/Engine/EditorBlueprintResources/StandardMacros.IsValid` _input_event_base_bp_temp
      (:`Is Valid`
        (`/Game/BP/common/component/input/base/input_event_base_BP.key_symbol_equal` _input_event_base_bp_temp)))))

(event `Key|Shift+H`
  (params (Key :type "Key Structure"))
  (bind _input_event_base_bp_temp (`self.input_event_base_BP_temp`))
  ;[1 1 1] char upper case
  (:`Pressed`
    (`/Engine/EditorBlueprintResources/StandardMacros.IsValid` _input_event_base_bp_temp
      (:`Is Valid`
        (`/Game/BP/common/component/input/base/input_event_base_BP.key_char_upper_H` _input_event_base_bp_temp)))))

(event `Key|H`
  (params (Key :type "Key Structure"))
  (bind _input_event_base_bp_temp (`self.input_event_base_BP_temp`))
  ;[1 1 1] char lower case
  (:`Pressed`
    (`/Engine/EditorBlueprintResources/StandardMacros.IsValid` _input_event_base_bp_temp
      (:`Is Valid`
        (`/Game/BP/common/component/input/base/input_event_base_BP.key_char_lower_h` _input_event_base_bp_temp)))))

(event `Key|Shift+Equals`
  (params (Key :type "Key Structure"))
  (bind _input_event_base_bp_temp (`self.input_event_base_BP_temp`))
  ;[1 1 1] symbol
  (:`Pressed`
    (`/Engine/EditorBlueprintResources/StandardMacros.IsValid` _input_event_base_bp_temp
      (:`Is Valid`
        (`/Game/BP/common/component/input/base/input_event_base_BP.key_symbol_plus` _input_event_base_bp_temp)))))

(event `Key|Shift+J`
  (params (Key :type "Key Structure"))
  (bind _input_event_base_bp_temp (`self.input_event_base_BP_temp`))
  ;[1 1 1] char upper case
  (:`Pressed`
    (`/Engine/EditorBlueprintResources/StandardMacros.IsValid` _input_event_base_bp_temp
      (:`Is Valid`
        (`/Game/BP/common/component/input/base/input_event_base_BP.key_char_upper_J` _input_event_base_bp_temp)))))

(event `Key|J`
  (params (Key :type "Key Structure"))
  (bind _input_event_base_bp_temp (`self.input_event_base_BP_temp`))
  ;[1 1 1] char lower case
  (:`Pressed`
    (`/Engine/EditorBlueprintResources/StandardMacros.IsValid` _input_event_base_bp_temp
      (:`Is Valid`
        (`/Game/BP/common/component/input/base/input_event_base_BP.key_char_lower_j` _input_event_base_bp_temp)))))

(event `Key|Shift+K`
  (params (Key :type "Key Structure"))
  (bind _input_event_base_bp_temp (`self.input_event_base_BP_temp`))
  ;[1 1 1] char upper case
  (:`Pressed`
    (`/Engine/EditorBlueprintResources/StandardMacros.IsValid` _input_event_base_bp_temp
      (:`Is Valid`
        (`/Game/BP/common/component/input/base/input_event_base_BP.key_char_upper_K` _input_event_base_bp_temp)))))

(event `Key|LeftBracket`
  (params (Key :type "Key Structure"))
  (bind _input_event_base_bp_temp (`self.input_event_base_BP_temp`))
  ;[1 1 1] symbol
  (:`Pressed`
    (`/Engine/EditorBlueprintResources/StandardMacros.IsValid` _input_event_base_bp_temp
      (:`Is Valid`
        (`/Game/BP/common/component/input/base/input_event_base_BP.key_symbol_bracketleft` _input_event_base_bp_temp)))))

(event `Key|K`
  (params (Key :type "Key Structure"))
  (bind _input_event_base_bp_temp (`self.input_event_base_BP_temp`))
  ;[1 1 1] char lower case
  (:`Pressed`
    (`/Engine/EditorBlueprintResources/StandardMacros.IsValid` _input_event_base_bp_temp
      (:`Is Valid`
        (`/Game/BP/common/component/input/base/input_event_base_BP.key_char_lower_k` _input_event_base_bp_temp)))))

(event `Key|Shift+L`
  (params (Key :type "Key Structure"))
  (bind _input_event_base_bp_temp (`self.input_event_base_BP_temp`))
  ;[1 1 1] char upper case
  (:`Pressed`
    (`/Engine/EditorBlueprintResources/StandardMacros.IsValid` _input_event_base_bp_temp
      (:`Is Valid`
        (`/Game/BP/common/component/input/base/input_event_base_BP.key_char_upper_L` _input_event_base_bp_temp)))))

(event `Key|L`
  (params (Key :type "Key Structure"))
  (bind _input_event_base_bp_temp (`self.input_event_base_BP_temp`))
  ;[1 1 1] char lower case
  (:`Pressed`
    (`/Engine/EditorBlueprintResources/StandardMacros.IsValid` _input_event_base_bp_temp
      (:`Is Valid`
        (`/Game/BP/common/component/input/base/input_event_base_BP.key_char_lower_l` _input_event_base_bp_temp)))))

(event `Key|RightBracket`
  (params (Key :type "Key Structure"))
  (bind _input_event_base_bp_temp (`self.input_event_base_BP_temp`))
  ;[1 1 1] symbol
  (:`Pressed`
    (`/Engine/EditorBlueprintResources/StandardMacros.IsValid` _input_event_base_bp_temp
      (:`Is Valid`
        (`/Game/BP/common/component/input/base/input_event_base_BP.key_symbol_bracketright` _input_event_base_bp_temp)))))

(event `Key|Shift+Z`
  (params (Key :type "Key Structure"))
  (bind _input_event_base_bp_temp (`self.input_event_base_BP_temp`))
  ;[1 1 1] char upper case
  (:`Pressed`
    (`/Engine/EditorBlueprintResources/StandardMacros.IsValid` _input_event_base_bp_temp
      (:`Is Valid`
        (`/Game/BP/common/component/input/base/input_event_base_BP.key_char_upper_Z` _input_event_base_bp_temp)))))

(event `Key|Z`
  (params (Key :type "Key Structure"))
  (bind _input_event_base_bp_temp (`self.input_event_base_BP_temp`))
  ;[1 1 1] char lower case
  (:`Pressed`
    (`/Engine/EditorBlueprintResources/StandardMacros.IsValid` _input_event_base_bp_temp
      (:`Is Valid`
        (`/Game/BP/common/component/input/base/input_event_base_BP.key_char_lower_z` _input_event_base_bp_temp)))))

(event `Key|Shift+LeftBracket`
  (params (Key :type "Key Structure"))
  (bind _input_event_base_bp_temp (`self.input_event_base_BP_temp`))
  ;[1 1 1] symbol
  (:`Pressed`
    (`/Engine/EditorBlueprintResources/StandardMacros.IsValid` _input_event_base_bp_temp
      (:`Is Valid`
        (`/Game/BP/common/component/input/base/input_event_base_BP.key_symbol_braceleft` _input_event_base_bp_temp)))))

(event `Key|Shift+X`
  (params (Key :type "Key Structure"))
  (bind _input_event_base_bp_temp (`self.input_event_base_BP_temp`))
  ;[1 1 1] char upper case
  (:`Pressed`
    (`/Engine/EditorBlueprintResources/StandardMacros.IsValid` _input_event_base_bp_temp
      (:`Is Valid`
        (`/Game/BP/common/component/input/base/input_event_base_BP.key_char_upper_X` _input_event_base_bp_temp)))))

(event `Key|Shift+RightBracket`
  (params (Key :type "Key Structure"))
  (bind _input_event_base_bp_temp (`self.input_event_base_BP_temp`))
  ;[1 1 1] symbol
  (:`Pressed`
    (`/Engine/EditorBlueprintResources/StandardMacros.IsValid` _input_event_base_bp_temp
      (:`Is Valid`
        (`/Game/BP/common/component/input/base/input_event_base_BP.key_symbol_braceright` _input_event_base_bp_temp)))))

(event `Key|X`
  (params (Key :type "Key Structure"))
  (bind _input_event_base_bp_temp (`self.input_event_base_BP_temp`))
  ;[1 1 1] char lower case
  (:`Pressed`
    (`/Engine/EditorBlueprintResources/StandardMacros.IsValid` _input_event_base_bp_temp
      (:`Is Valid`
        (`/Game/BP/common/component/input/base/input_event_base_BP.key_char_lower_x` _input_event_base_bp_temp)))))

(event `Key|Shift+C`
  (params (Key :type "Key Structure"))
  (bind _input_event_base_bp_temp (`self.input_event_base_BP_temp`))
  ;[1 1 1] char upper case
  (:`Pressed`
    (`/Engine/EditorBlueprintResources/StandardMacros.IsValid` _input_event_base_bp_temp
      (:`Is Valid`
        (`/Game/BP/common/component/input/base/input_event_base_BP.key_char_upper_C` _input_event_base_bp_temp)))))

(event `Key|Backslash`
  (params (Key :type "Key Structure"))
  (bind _input_event_base_bp_temp (`self.input_event_base_BP_temp`))
  ;[1 1 1] symbol
  (:`Pressed`
    (`/Engine/EditorBlueprintResources/StandardMacros.IsValid` _input_event_base_bp_temp
      (:`Is Valid`
        (`/Game/BP/common/component/input/base/input_event_base_BP.key_symbol_backslash` _input_event_base_bp_temp)))))

(event `Key|C`
  (params (Key :type "Key Structure"))
  (bind _input_event_base_bp_temp (`self.input_event_base_BP_temp`))
  ;[1 1 1] char lower case
  (:`Pressed`
    (`/Engine/EditorBlueprintResources/StandardMacros.IsValid` _input_event_base_bp_temp
      (:`Is Valid`
        (`/Game/BP/common/component/input/base/input_event_base_BP.key_char_lower_c` _input_event_base_bp_temp)))))

(event `Key|Shift+V`
  (params (Key :type "Key Structure"))
  (bind _input_event_base_bp_temp (`self.input_event_base_BP_temp`))
  ;[1 1 1] char upper case
  (:`Pressed`
    (`/Engine/EditorBlueprintResources/StandardMacros.IsValid` _input_event_base_bp_temp
      (:`Is Valid`
        (`/Game/BP/common/component/input/base/input_event_base_BP.key_char_upper_V` _input_event_base_bp_temp)))))

(event `Key|V`
  (params (Key :type "Key Structure"))
  (bind _input_event_base_bp_temp (`self.input_event_base_BP_temp`))
  ;[1 1 1] char lower case
  (:`Pressed`
    (`/Engine/EditorBlueprintResources/StandardMacros.IsValid` _input_event_base_bp_temp
      (:`Is Valid`
        (`/Game/BP/common/component/input/base/input_event_base_BP.key_char_lower_v` _input_event_base_bp_temp)))))

(event `Key|Shift+Backslash`
  (params (Key :type "Key Structure"))
  (bind _input_event_base_bp_temp (`self.input_event_base_BP_temp`))
  ;[1 1 1] symbol
  (:`Pressed`
    (`/Engine/EditorBlueprintResources/StandardMacros.IsValid` _input_event_base_bp_temp
      (:`Is Valid`
        (`/Game/BP/common/component/input/base/input_event_base_BP.key_symbol_bar` _input_event_base_bp_temp)))))

(event `Key|Shift+B`
  (params (Key :type "Key Structure"))
  (bind _input_event_base_bp_temp (`self.input_event_base_BP_temp`))
  ;[1 1 1] char upper case
  (:`Pressed`
    (`/Engine/EditorBlueprintResources/StandardMacros.IsValid` _input_event_base_bp_temp
      (:`Is Valid`
        (`/Game/BP/common/component/input/base/input_event_base_BP.key_char_upper_B` _input_event_base_bp_temp)))))

(event `Key|B`
  (params (Key :type "Key Structure"))
  (bind _input_event_base_bp_temp (`self.input_event_base_BP_temp`))
  ;[1 1 1] char lower case
  (:`Pressed`
    (`/Engine/EditorBlueprintResources/StandardMacros.IsValid` _input_event_base_bp_temp
      (:`Is Valid`
        (`/Game/BP/common/component/input/base/input_event_base_BP.key_char_lower_b` _input_event_base_bp_temp)))))

(event `Key|Semicolon`
  (params (Key :type "Key Structure"))
  (bind _input_event_base_bp_temp (`self.input_event_base_BP_temp`))
  ;[1 1 1] symbol
  (:`Pressed`
    (`/Engine/EditorBlueprintResources/StandardMacros.IsValid` _input_event_base_bp_temp
      (:`Is Valid`
        (`/Game/BP/common/component/input/base/input_event_base_BP.key_symbol_semicolon` _input_event_base_bp_temp)))))

(event `Key|Shift+N`
  (params (Key :type "Key Structure"))
  (bind _input_event_base_bp_temp (`self.input_event_base_BP_temp`))
  ;[1 1 1] char upper case
  (:`Pressed`
    (`/Engine/EditorBlueprintResources/StandardMacros.IsValid` _input_event_base_bp_temp
      (:`Is Valid`
        (`/Game/BP/common/component/input/base/input_event_base_BP.key_char_upper_N` _input_event_base_bp_temp)))))

(event `Key|N`
  (params (Key :type "Key Structure"))
  (bind _input_event_base_bp_temp (`self.input_event_base_BP_temp`))
  ;[1 1 1] char lower case
  (:`Pressed`
    (`/Engine/EditorBlueprintResources/StandardMacros.IsValid` _input_event_base_bp_temp
      (:`Is Valid`
        (`/Game/BP/common/component/input/base/input_event_base_BP.key_char_lower_n` _input_event_base_bp_temp)))))

(event `Key|Shift+Semicolon`
  (params (Key :type "Key Structure"))
  (bind _input_event_base_bp_temp (`self.input_event_base_BP_temp`))
  ;[1 1 1] symbol
  (:`Pressed`
    (`/Engine/EditorBlueprintResources/StandardMacros.IsValid` _input_event_base_bp_temp
      (:`Is Valid`
        (`/Game/BP/common/component/input/base/input_event_base_BP.key_symbol_colon` _input_event_base_bp_temp)))))

(event `Key|Shift+M`
  (params (Key :type "Key Structure"))
  (bind _input_event_base_bp_temp (`self.input_event_base_BP_temp`))
  ;[1 1 1] char upper case
  (:`Pressed`
    (`/Engine/EditorBlueprintResources/StandardMacros.IsValid` _input_event_base_bp_temp
      (:`Is Valid`
        (`/Game/BP/common/component/input/base/input_event_base_BP.key_char_upper_M` _input_event_base_bp_temp)))))

(event `Key|M`
  (params (Key :type "Key Structure"))
  (bind _input_event_base_bp_temp (`self.input_event_base_BP_temp`))
  ;[1 1 1] char lower case
  (:`Pressed`
    (`/Engine/EditorBlueprintResources/StandardMacros.IsValid` _input_event_base_bp_temp
      (:`Is Valid`
        (`/Game/BP/common/component/input/base/input_event_base_BP.key_char_lower_m` _input_event_base_bp_temp)))))

(event `Key|Apostrophe`
  (params (Key :type "Key Structure"))
  (bind _input_event_base_bp_temp (`self.input_event_base_BP_temp`))
  ;[1 1 1] symbol
  (:`Pressed`
    (`/Engine/EditorBlueprintResources/StandardMacros.IsValid` _input_event_base_bp_temp
      (:`Is Valid`
        (`/Game/BP/common/component/input/base/input_event_base_BP.key_symbol_quote` _input_event_base_bp_temp)))))

(event `Key|Shift+Quote`
  (params (Key :type "Key Structure"))
  (bind _input_event_base_bp_temp (`self.input_event_base_BP_temp`))
  ;[1 1 1] symbol
  (:`Pressed`
    (`/Engine/EditorBlueprintResources/StandardMacros.IsValid` _input_event_base_bp_temp :!label _label_2
      (:`Is Valid`
        (`/Game/BP/common/component/input/base/input_event_base_BP.key_symbol_doublequote` _input_event_base_bp_temp)))))

(event `Key|Shift+Apostrophe`
  (params (Key :type "Key Structure"))
  ;[1 1 1] symbol
  (:`Pressed`
    (goto _label_2)))

(event `Key|Comma`
  (params (Key :type "Key Structure"))
  (bind _input_event_base_bp_temp (`self.input_event_base_BP_temp`))
  ;[1 1 1] symbol
  (:`Pressed`
    (`/Engine/EditorBlueprintResources/StandardMacros.IsValid` _input_event_base_bp_temp
      (:`Is Valid`
        (`/Game/BP/common/component/input/base/input_event_base_BP.key_symbol_comma` _input_event_base_bp_temp)))))

(event `Key|Shift+Comma`
  (params (Key :type "Key Structure"))
  (bind _input_event_base_bp_temp (`self.input_event_base_BP_temp`))
  ;[1 1 1] symbol
  (:`Pressed`
    (`/Engine/EditorBlueprintResources/StandardMacros.IsValid` _input_event_base_bp_temp
      (:`Is Valid`
        (`/Game/BP/common/component/input/base/input_event_base_BP.key_symbol_less` _input_event_base_bp_temp)))))

(event `Key|Period`
  (params (Key :type "Key Structure"))
  (bind _input_event_base_bp_temp (`self.input_event_base_BP_temp`))
  ;[1 1 1] symbol
  (:`Pressed`
    (`/Engine/EditorBlueprintResources/StandardMacros.IsValid` _input_event_base_bp_temp
      (:`Is Valid`
        (`/Game/BP/common/component/input/base/input_event_base_BP.key_symbol_dot` _input_event_base_bp_temp)))))

(event `Key|Shift+Period`
  (params (Key :type "Key Structure"))
  (bind _input_event_base_bp_temp (`self.input_event_base_BP_temp`))
  ;[1 1 1] symbol
  (:`Pressed`
    (`/Engine/EditorBlueprintResources/StandardMacros.IsValid` _input_event_base_bp_temp
      (:`Is Valid`
        (`/Game/BP/common/component/input/base/input_event_base_BP.key_symbol_greater` _input_event_base_bp_temp)))))

(event `Key|Slash`
  (params (Key :type "Key Structure"))
  (bind _input_event_base_bp_temp (`self.input_event_base_BP_temp`))
  ;[1 1 1] symbol
  (:`Pressed`
    (`/Engine/EditorBlueprintResources/StandardMacros.IsValid` _input_event_base_bp_temp
      (:`Is Valid`
        (`/Game/BP/common/component/input/base/input_event_base_BP.key_symbol_slash` _input_event_base_bp_temp)))))

(event `Key|Shift+Slash`
  (params (Key :type "Key Structure"))
  (bind _input_event_base_bp_temp (`self.input_event_base_BP_temp`))
  ;[1 1 1] symbol
  (:`Pressed`
    (`/Engine/EditorBlueprintResources/StandardMacros.IsValid` _input_event_base_bp_temp
      (:`Is Valid`
        (`/Game/BP/common/component/input/base/input_event_base_BP.key_symbol_questionmark` _input_event_base_bp_temp)))))

(event `Key|SpaceBar`
  (params (Key :type "Key Structure"))
  (bind _input_event_base_bp_temp (`self.input_event_base_BP_temp`))
  ;[1 1 1] symbol
  (:`Pressed`
    (`/Engine/EditorBlueprintResources/StandardMacros.IsValid` _input_event_base_bp_temp
      (:`Is Valid`
        (`/Game/BP/common/component/input/base/input_event_base_BP.key_symbol_space_bar` _input_event_base_bp_temp)))))

(event `Key|BackSpace`
  (params (Key :type "Key Structure"))
  (bind _input_event_base_bp_temp (`self.input_event_base_BP_temp`))
  ;[1 1 1] symbol
  (:`Pressed`
    (`/Engine/EditorBlueprintResources/StandardMacros.IsValid` _input_event_base_bp_temp
      (:`Is Valid`
        (`/Game/BP/common/component/input/base/input_event_base_BP.key_symbol_backspace` _input_event_base_bp_temp)))))

(fn `init_function`)

(fn `UserConstructionScript`)